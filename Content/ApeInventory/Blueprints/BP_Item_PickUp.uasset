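; BP_Item_PickUp is a spinning world pickup that adds its item to the player's inventory on overlap.
; Tick rotates the root around yaw at a frame-rate-independent speed.
; Collider overlap by the player pawn gets the inventory through an interface message, calls AddItem and destroys the pickup only on success.
; Seticontotexture applies the item's icon via a dynamic material instance, but nothing in this graph calls it.
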(event `self.ReceiveBeginPlay`)

(event `Set icon to texture`
  (bind _staticmesh (`self.StaticMesh`))
  (bind _item (`self.Item`))
  ;[1 1 1] Dynamic Texture
  (bind _returnvalue (`PrimitiveComponent.CreateDynamicMaterialInstance` _staticmesh 0 "/Game/ApeInventory/Materials/MAT_DynamicTexture.MAT_DynamicTexture" "None"))
  (bind _texture2d (`/Game/ApeInventory/Blueprints/FL_ItemUtil.FL_GetItemIcon` (`Item.ItemID` _item) (`Item.ItemType` _item)))
  (`MaterialInstanceDynamic.SetTextureParameterValue` _returnvalue "Normal" _texture2d)
  (`PrimitiveComponent.SetMaterial` _staticmesh 0 _returnvalue))

(event `self.ReceiveTick`
  (params (DeltaSeconds :type "Float (single-precision)"))
  ;[1 1 1] Rotator
  (`SceneComponent.K2_AddLocalRotation` (`self.DefaultSceneRoot`) (`KismetMathLibrary.MakeRotator` 0.0 0.0 (* 40 DeltaSeconds)) false false))

(event `self.Collider.OnComponentBeginOverlap`
  (params (OverlappedComponent :type "PrimitiveComponent Object Reference") (OtherActor :type "Actor Object Reference") (OtherComp :type "PrimitiveComponent Object Reference") (OtherBodyIndex :type Integer) (bFromSweep :type Boolean) (SweepResult :type "HitResult Structure (by ref)"))
  (bind _returnvalue (`GameplayStatics.GetPlayerPawn` 0))
  ;[1 1 1] Add item to player character
  (if (== OtherActor _returnvalue)
    (bind _inventorycomponent (message `/Game/ApeInventory/Interface/BPI_InventoryActor.INT_GetInventory` _returnvalue))
    (bind _returnvalue_2 (`InventoryComponent.AddItem` _inventorycomponent (`self.Item`)))
    ;[1 1 1] Destroy this pickup
    (if _returnvalue_2
      (`self.K2_DestroyActor`))))

(fn `UserConstructionScript`)