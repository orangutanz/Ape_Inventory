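; Blueprint function library for the ApeInventory system that looks up item definitions and icons by item ID.
; Separate getters read rows from the Consumable, Equipment and MiscItem data tables, returning only when the row is found.
; The icon function switches on item type, calls the matching getter, then synchronously loads the soft icon reference and casts it to Texture2D.
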(fn `FL_GetConsumableInfo`
  (params (ItemID :type Name))
  (returns (`Data Table` :type "DataTable Object Reference") (`Out Row` :type "/Game/ApeInventory/Database/ST_Consumable Structure"))
  (bind _returnvalue (`|GetDataTableRow` "/Game/ApeInventory/Database/DT_Consumable.DT_Consumable" ItemID)
    (:`then`
      (return "/Game/ApeInventory/Database/DT_Consumable.DT_Consumable" _returnvalue))))

(fn `FL_GetEquipmentInfo`
  (params (ItemID :type Name))
  (returns (`Data Table` :type "DataTable Object Reference") (`Out Row` :type "/Game/ApeInventory/Database/ST_Equipment Structure"))
  (bind _returnvalue (`|GetDataTableRow` "/Game/ApeInventory/Database/DT_Equipment.DT_Equipment" ItemID)
    (:`then`
      (return "/Game/ApeInventory/Database/DT_Equipment.DT_Equipment" _returnvalue))))

(fn `FL_GetItemIcon`
  (params (ItemID :type Name) (ItemType :type "ItemType Enum" :default "Consumable"))
  (returns (Texture2D :type "Texture2D Object Reference"))
  (switch `ItemType` ItemType
    (:`Consumable`
      (bind (_data_table _out_row) (`self.FL_GetConsumableInfo` ItemID))
      (bind _returnvalue (`KismetSystemLibrary.LoadAsset_Blocking` (`.Icon_23_EDE83E614CDA31987D5B66B5051B9958` (break `/Game/ApeInventory/Database/ST_ItemBase` (`.ItemBase_33_3C39835B40E7B955698D3FAC2CBF52CA` (break `/Game/ApeInventory/Database/ST_Consumable` _out_row))))))
      (bind _astexture_2d (cast `Texture2D` _returnvalue))
      (return _astexture_2d))
    (:`Equipment`
      (bind (_data_table_2 _out_row_2) (`self.FL_GetEquipmentInfo` null ItemID))
      (bind _returnvalue_2 (`KismetSystemLibrary.LoadAsset_Blocking` (`.Icon_23_EDE83E614CDA31987D5B66B5051B9958` (break `/Game/ApeInventory/Database/ST_ItemBase` (`.ItemBase_28_068767E043BEEE5F67A81D9B6186AD07` (break `/Game/ApeInventory/Database/ST_Equipment` _out_row_2))))))
      (bind _astexture_2d_2 (cast `Texture2D` _returnvalue_2))
      (return _astexture_2d_2))
    (:`Misc`
      (bind (_data_table_3 _out_row_3) (`self.FL_GetMiscItemInfo` ItemID))
      (bind _returnvalue_3 (`KismetSystemLibrary.LoadAsset_Blocking` (`.Icon_23_EDE83E614CDA31987D5B66B5051B9958` (break `/Game/ApeInventory/Database/ST_ItemBase` _out_row_3))))
      (bind _astexture_2d_3 (cast `Texture2D` _returnvalue_3))
      (return _astexture_2d_3))))

(fn `FL_GetMiscItemInfo`
  (params (ItemID :type Name))
  (returns (`Data Table` :type "DataTable Object Reference") (`Out Row` :type "/Game/ApeInventory/Database/ST_ItemBase Structure"))
  (bind _returnvalue (`|GetDataTableRow` "/Game/ApeInventory/Database/DT_MiscItem.DT_MiscItem" ItemID)
    (:`then`
      (return "/Game/ApeInventory/Database/DT_MiscItem.DT_MiscItem" _returnvalue))))