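; BP_PickUp is an item pickup that spins in the world and gives its Item to the player on touch.
; Tick rotates the root around yaw at a frame-rate-independent speed.
; Collider overlap with Ape_TopDownCharacter adds the Item to that character's inventory and destroys the pickup only if the add succeeds.
; A custom event, not called here, shows the item icon on the mesh through a dynamic material instance.
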(event `self.ReceiveBeginPlay`)

(event `Set icon to texture`
  (bind _staticmesh (`self.StaticMesh`))
  ;[1 1 1] Dynamic Texture
  (bind _returnvalue (`PrimitiveComponent.CreateDynamicMaterialInstance` _staticmesh 0 "/Game/ApeInventory/Materials/MAT_DynamicTexture.MAT_DynamicTexture" "None"))
  (`MaterialInstanceDynamic.SetTextureParameterValue` _returnvalue "Normal" (`Item.Icon` (`self.Item`)))
  (`PrimitiveComponent.SetMaterial` _staticmesh 0 _returnvalue))

(event `self.ReceiveTick`
  (params (DeltaSeconds :type "Float (single-precision)"))
  ;[1 1 1] Rotator
  (`SceneComponent.K2_AddLocalRotation` (`self.DefaultSceneRoot`) (`KismetMathLibrary.MakeRotator` 0.0 0.0 (* 40 DeltaSeconds)) false false))

(event `self.Collider.OnComponentBeginOverlap`
  (params (OverlappedComponent :type "PrimitiveComponent Object Reference") (OtherActor :type "Actor Object Reference") (OtherComp :type "PrimitiveComponent Object Reference") (OtherBodyIndex :type Integer) (bFromSweep :type Boolean) (SweepResult :type "HitResult Structure (by ref)"))
  ;[1 1 1] Add item to player character
  (bind _astop_down_character (cast `/Game/ApeInventory/Blueprints/Ape_TopDownCharacter` OtherActor))
  (bind _returnvalue (`InventoryComponent.AddItem` (`Ape_InventoryCharacter.Inventory` _astop_down_character) (`self.Item`)))
  ;[1 1 1] Destroy this pickup
  (if _returnvalue
    (`self.K2_DestroyActor`)))

(fn `UserConstructionScript`)