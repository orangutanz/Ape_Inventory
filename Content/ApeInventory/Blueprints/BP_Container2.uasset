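; BP_Container2 is a world container that shows its inventory UI while the player's pawn is inside its Box trigger.
; Overlap begin and end send interface messages to the pawn to add or remove the container widget and toggle the player's inventory widget.
; GetContainerWidget lazily creates and caches a WBP_Container, assigning it this container's Inventory.
; Disconnected nodes hold unused direct viewport and inventory initialization logic.
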(event `self.ReceiveBeginPlay`)

(event `self.Box.OnComponentBeginOverlap`
  (params (OverlappedComponent :type "PrimitiveComponent Object Reference") (OtherActor :type "Actor Object Reference") (OtherComp :type "PrimitiveComponent Object Reference") (OtherBodyIndex :type Integer) (bFromSweep :type Boolean) (SweepResult :type "HitResult Structure (by ref)"))
  (bind _returnvalue (`GameplayStatics.GetPlayerPawn` 0))
  ;[1 1 1] Toggle player's inventory widget. Add/remove this container's widget
  (if (== OtherActor _returnvalue)
    (bind _widget (`self.GetContainerWidget`))
    (message `/Game/ApeInventory/Blueprints/BPI_InventoryActor.INT_AddContainerWidget` _returnvalue _widget)
    (message `/Game/ApeInventory/Blueprints/BPI_InventoryActor.INT_ToggleInventoryWidget` _returnvalue true) ; Optional
  ))

(event `self.Box.OnComponentEndOverlap`
  (params (OverlappedComponent :type "PrimitiveComponent Object Reference") (OtherActor :type "Actor Object Reference") (OtherComp :type "PrimitiveComponent Object Reference") (OtherBodyIndex :type Integer))
  (bind _returnvalue (`GameplayStatics.GetPlayerPawn` 0))
  ;[1 1 1] Toggle player's inventory widget. Add/remove this container's widget
  (if (== _returnvalue OtherActor)
    (bind _widget (`self.GetContainerWidget`))
    (message `/Game/ApeInventory/Blueprints/BPI_InventoryActor.INT_RemoveContainerWidget` _returnvalue _widget)
    (message `/Game/ApeInventory/Blueprints/BPI_InventoryActor.INT_ToggleInventoryWidget` _returnvalue false) ; optional
  ))

(fn `GetContainerWidget`
  (returns (Widget :type "UserWidget Object Reference"))
  (`/Engine/EditorBlueprintResources/StandardMacros.IsValid` (`self.Container Widget`)
    (:`Is Valid`
      _)
    (:`Is Not Valid`
      (bind _returnvalue (`|CreateWidget` "/Game/ApeInventory/Widgets/WBP_Container.WBP_Container_C" (`GameplayStatics.GetPlayerController` 0)))
      (bind _output_get (set `self.Container Widget` _returnvalue))
      (set `/Game/ApeInventory/Widgets/WBP_Container.Inventory` (`self.Inventory`) _output_get)))
  (return (`self.Container Widget`)))

(fn `UserConstructionScript`)