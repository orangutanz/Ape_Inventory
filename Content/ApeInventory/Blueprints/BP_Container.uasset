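; BP_Container is a world container that opens its inventory UI when an Ape_TopDownCharacter enters its Box trigger.
; On BeginPlay it creates a WBP_Container widget for player 0 and hands it the container's Inventory.
; On overlap it toggles the player's inventory, initializes the container widget, cross-links it with the player's inventory widget and adds it to the viewport.
; On exit it closes both and clears the player inventory link.
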(event `self.ReceiveBeginPlay`
  (bind _returnvalue (`|CreateWidget` "/Game/ApeInventory/Widgets/WBP_Container.WBP_Container_C" (`GameplayStatics.GetPlayerController` 0)))
  (bind _output_get (set `self.Container Widget` _returnvalue))
  (set `/Game/ApeInventory/Widgets/WBP_Container.Inventory` (`self.Inventory`) _output_get))

(event `self.Box.OnComponentBeginOverlap`
  (params (OverlappedComponent :type "PrimitiveComponent Object Reference") (OtherActor :type "Actor Object Reference") (OtherComp :type "PrimitiveComponent Object Reference") (OtherBodyIndex :type Integer) (bFromSweep :type Boolean) (SweepResult :type "HitResult Structure (by ref)"))
  (bind _container_widget (`self.Container Widget`))
  ;[1 1 1] Toggle player's inventory widget
  (bind _astop_down_character (cast `/Game/ApeInventory/Blueprints/Ape_TopDownCharacter` OtherActor))
  (`/Game/ApeInventory/Blueprints/Ape_TopDownCharacter.Toggle Invnetory` _astop_down_character true)
  ;[1 1 1] Create a container widget on player
  (`/Game/ApeInventory/Widgets/WBP_Container.Initialize Inventory` _container_widget (`self.Inventory`))
  (bind _inventorywidget (`/Game/ApeInventory/Blueprints/Ape_TopDownCharacter.InventoryWidget` _astop_down_character))
  (set `/Game/ApeInventory/Widgets/WBP_Inventory.Target Container` _container_widget _inventorywidget)
  (set `/Game/ApeInventory/Widgets/WBP_Container.UserInvntory` (`/Game/ApeInventory/Widgets/WBP_Inventory.Inventory` _inventorywidget) _container_widget)
  (`UserWidget.AddToViewport` _container_widget 0))

(event `self.Box.OnComponentEndOverlap`
  (params (OverlappedComponent :type "PrimitiveComponent Object Reference") (OtherActor :type "Actor Object Reference") (OtherComp :type "PrimitiveComponent Object Reference") (OtherBodyIndex :type Integer))
  ;[1 1 1] Toggle player's inventory widget
  (bind _astop_down_character (cast `/Game/ApeInventory/Blueprints/Ape_TopDownCharacter` OtherActor))
  (`/Game/ApeInventory/Blueprints/Ape_TopDownCharacter.Toggle Invnetory` _astop_down_character false)
  (set `/Game/ApeInventory/Widgets/WBP_Container.UserInvntory` null (`self.Container Widget`))
  (`Widget.RemoveFromParent` (`self.Container Widget`)))

(fn `UserConstructionScript`)