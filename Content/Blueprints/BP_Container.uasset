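; BP_Container is a world container that shows its inventory to the player while they stand inside its Box trigger.
; On overlap by a TopDownCharacter, it toggles that character's inventory on, then creates a WBP_Container widget for player 0, initializes it with the container's Inventory and adds it to the viewport.
; Ending the overlap toggles the character's inventory off and removes the container widget.
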(event `self.Box.OnComponentBeginOverlap`
  (params (OverlappedComponent :type "PrimitiveComponent Object Reference") (OtherActor :type "Actor Object Reference") (OtherComp :type "PrimitiveComponent Object Reference") (OtherBodyIndex :type Integer) (bFromSweep :type Boolean) (SweepResult :type "HitResult Structure (by ref)"))
  ;[1 1 1] Toggle player's inventory widget
  (bind _astop_down_character (cast `/Game/Blueprints/TopDownCharacter` OtherActor))
  (`/Game/Blueprints/TopDownCharacter.Toggle Invnetory` _astop_down_character true)
  ;[1 1 1] Create a container widget on player
  (bind _returnvalue (`|CreateWidget` "/Game/Widgets/WBP_Container.WBP_Container_C" (`GameplayStatics.GetPlayerController` 0)))
  (bind _output_get (set `/Game/Widgets/WBP_Container.Inventory` (`self.Inventory`) _returnvalue))
  (`/Game/Widgets/WBP_Container.Initialize Inventory` _returnvalue _output_get)
  (`UserWidget.AddToViewport` _returnvalue 0))

(event `self.Box.OnComponentEndOverlap`
  (params (OverlappedComponent :type "PrimitiveComponent Object Reference") (OtherActor :type "Actor Object Reference") (OtherComp :type "PrimitiveComponent Object Reference") (OtherBodyIndex :type Integer))
  ;[1 1 1] Toggle player's inventory widget
  (bind _astop_down_character (cast `/Game/Blueprints/TopDownCharacter` OtherActor))
  (`/Game/Blueprints/TopDownCharacter.Toggle Invnetory` _astop_down_character false)
  (`Widget.RemoveFromParent` (stale `self.Box.OnComponentBeginOverlap` _returnvalue)))

(fn `UserConstructionScript`)